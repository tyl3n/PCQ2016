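; BP_Shockwave is a shockwave actor that pairs a particle effect with collision detection against other actors.
; On BeginPlay it feeds RadiusGrowRate and MaxLifeSpan into the particle system as velocity and lifespan.
; Each Tick it passes every actor in the world to DetectCollisionForOneActor, defined outside these graphs, and colors particles orange for attacks, white otherwise.
; Unconnected nodes remain for destroying the particles and drawing a debug cylinder.
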(event `self.ReceiveBeginPlay`
  (bind _particlesystem (`self.ParticleSystem`))
  (`ParticleSystemComponent.SetFloatParameter` _particlesystem "Velocity" (`self.radiusGrowRate`))
  (`ParticleSystemComponent.SetFloatParameter` _particlesystem "Lifespan" (`self.maxLifeSpan`)))

(event `self.ReceiveActorBeginOverlap`
  (params (OtherActor :type "Actor Object Reference")))

(event `self.ReceiveTick`
  (params (DeltaSeconds :type "Float (single-precision)"))
  (bind _particlesystem (`self.ParticleSystem`))
  (bind _outactors (`GameplayStatics.GetAllActorsOfClass` "/Script/Engine.Actor"))
  (for _array_element _outactors
    (`self.detectCollisionForOneActor` _array_element)
    (if (`self.isAttack`)
      (`ParticleSystemComponent.SetColorParameter` _particlesystem "ParticleColor" (struct :`R` 1.0 :`G` 0.589154 :`B` 0.14765 :`A` 1.0))
      (else
        (`ParticleSystemComponent.SetColorParameter` _particlesystem "ParticleColor" (struct :`R` 1.0 :`G` 1.0 :`B` 1.0 :`A` 1.0))))))

(fn `UserConstructionScript`)