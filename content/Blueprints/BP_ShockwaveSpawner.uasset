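; Spawner actor that periodically emits a shockwave at its own transform, with a thunder clap sound and a particle flash.
; A looping timer started on BeginPlay calls CreateShockwave, which plays the sound, shows the particle system and spawns a BP_Shockwave with the spawner's configured strength.
; Tick watches for the visible particle system and hides it after a short Delay, so the effect shows only briefly per pulse.
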(event `self.ReceiveBeginPlay`
  (`KismetSystemLibrary.K2_SetTimer` null "CreateShockwave" 10.0 true))

(event `self.ReceiveTick`
  (params (DeltaSeconds :type "Float (single-precision)"))
  (bind _particlesystem (`self.ParticleSystem`))
  (if (`SceneComponent.IsVisible` _particlesystem)
    (`KismetSystemLibrary.Delay` 0.2)
    (`SceneComponent.SetVisibility` _particlesystem false true)))

(fn `CreateShockwave`
  (`GameplayStatics.PlaySoundAtLocation` "/Game/Sounds/Thunder_Clap-SoundBible_com-1913038465.Thunder_Clap-SoundBible_com-1913038465")
  (`SceneComponent.SetVisibility` (`self.ParticleSystem`) true true)
  (bind _returnvalue (`|SpawnActorFromClass` "/Game/Blueprints/BP_Shockwave.BP_Shockwave_C" (`self.GetTransform`) "AlwaysSpawn" "OverrideRootScale"))
  (set `Shockwave.strength` (`self.StrengthOfShockwave`) _returnvalue))

(fn `UserConstructionScript`)